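; BP_CaveCritter is a cave creature that wakes on seeing the player character, flees and vanishes.
; PawnSensing fires a one-shot sequence that swaps in a cell-shader material and plays an awake montage before starting RunAway.
; RunAway repeatedly uses AIMoveTo toward points away from the player at its own height, re-triggering on success or failure.
; Timed delays then swap to an invisible material, activate Niagara and destroy the actor.
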(event OnSeePawn(PawnSensing)
  (params (Pawn :type Pawn%20Object%20Reference))
  (bind _mesh (Variables|Character|GetMesh))
  (if (== Pawn (Variables|Default|GetChar%20Ref))
    (Utilities|FlowControl|DoOnce false
      (:Completed
        (Rendering|Material|SetMaterial (Variables|Character|GetMesh) 0 "/Game/Assets/3DMeshes/CaveCritter/MI_CellshaderCaveCritter.MI_CellshaderCaveCritter")
        (Animation|PlayAnimMontage "/Game/Assets/3DMeshes/CaveCritter/AM_CaveCritter_Awake.AM_CaveCritter_Awake" 1.0 "None")
        (Utilities|FlowControl|Delay 1.0)
        (CallFunction|RunAway)
        (Utilities|FlowControl|Delay 2.5)
        (Rendering|Material|SetMaterial _mesh 0 "/Game/Assets/Materials/NewFolder/M_InvisibleTest.M_InvisibleTest")
        (Rendering|Material|SetMaterial _mesh 1 "/Game/Assets/Materials/NewFolder/M_InvisibleTest.M_InvisibleTest")
        (Components|Activation|Activate (Variables|Default|GetNiagara) false)
        (Utilities|FlowControl|Delay 1.0)
        (Actor|DestroyActor)))))

(event Custom|Run%20Away
  (bind _returnvalue (Transformation|GetActorLocation))
  (bind _char_ref (Variables|Default|GetChar%20Ref))
  (bind _returnvalue_2 (Transformation|GetActorLocation _char_ref))
  (bind _returnvalue_3 (Math|Rotator|FindLookatRotation _returnvalue _returnvalue_2))
  (bind _returnvalue_4 (Math|Vector|GetForwardVector _returnvalue_3))
  (bind _returnvalue_5 (* _returnvalue_4 -5e+02))
  (bind _returnvalue_6 (+ _returnvalue _returnvalue_5))
  (bind (_x _y) (Math|Vector|BreakVector _returnvalue_6))
  (AI|AIMoveTo self (Math|Vector|MakeVector _x _y (.Z (Math|Vector|BreakVector _returnvalue))) 0 5.0 false
    (:OnSuccess
      _)
    (:OnFail
      _))
  (CallFunction|RunAway))

(event EventBeginPlay
  (bind _asbp_third_person_character (Utilities|Casting|CastToBP_ThirdPersonCharacter (Game|GetPlayerCharacter 0)))
  (Variables|Default|SetChar%20Ref _asbp_third_person_character))

(event EventTick
  (params (DeltaSeconds :type Float%20%28single-precision%29)))

(fn ConstructionScript)