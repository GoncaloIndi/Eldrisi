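; BP_LevelTransition is a trigger box that plays an ending cutscene and moves the player to the Eldrisi_level1 map.
; When BP_ThirdPersonCharacter overlaps the box, a DoOnce fades screen and audio out and removes all widgets.
; After a short delay it pauses the Amb audio bus, shows WBP_Cutscene2 and disables input.
; A fixed delay, rather than a widget callback, times the level load.
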(event OnComponentBeginOverlap(Box)
  (params (OverlappedComponent :type Primitive%20Component%20Object%20Reference) (OtherActor :type Actor%20Object%20Reference) (OtherComp :type Primitive%20Component%20Object%20Reference) (OtherBodyIndex :type Integer) (bFromSweep :type Boolean) (SweepResult :type Hit%20Result%20Structure%20%28by%20ref%29))
  (bind _returnvalue (Game|GetPlayerController 0))
  (Utilities|Casting|CastToBP_ThirdPersonCharacter OtherActor)
  (Utilities|FlowControl|DoOnce false
    (:Completed
      (CameraFades|StartCameraFade :self (Game|GetPlayerCameraManager 0) :ToAlpha 1.0 :Duration 3.0 :bShouldFadeAudio true :bHoldWhenFinished true)
      (Viewport|RemoveAllWidgets)
      (Utilities|FlowControl|RetriggerableDelay 3.5)
      (Class|FMODBlueprintStatics|BusSetPaused "/Game/Fmod/Buses/Amb.Amb" true)
      (bind _returnvalue_2 (UserInterface|CreateWidget "/Game/Assets/UI_Menu/Cutscenes/Cutscene2/WBP_Cutscene2.WBP_Cutscene2_C"))
      (UserInterface|Viewport|AddtoViewport _returnvalue_2 0)
      (Input|DisableInput _returnvalue 0)
      (Utilities|FlowControl|Delay 27.0)
      (Game|OpenLevel(byName) "Eldrisi_level1")
      (Input|EnableInput _returnvalue 0))))

(fn ConstructionScript)