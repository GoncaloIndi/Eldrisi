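; Small enemy that shoots at pawns it sees and breaks apart on death.
; Pawn sensing starts a yaw-tracking loop via recursive Delay and a gated attack firing montage-timed projectiles, with impulse scaled by target distance.
; Damage plays a hit montage or, at zero health, swaps the mesh for physics pieces, spawns a head and destroys the actor.
; Events also cover healing and AI movement, where RunFromPlayer actually moves toward the player.
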(event OnSeePawn(PawnSensing)
  (params (Pawn :type Pawn%20Object%20Reference))
  (Variables|Default|SetIsSeeingPlayer true)
  (CallFunction|ShootPlayer))

(event Custom|Shoot%20Player
  (Utilities|FlowControl|Sequence
    (:then_0
      (CallFunction|FacePlayer))
    (:then_1
      (Utilities|FlowControl|DoOnce false :!label _label
        (:Completed
          ;[1 1 1] Shoot
          (if (Variables|Default|GetCanShootPlayer)
            (Animation|PlayAnimMontage "/Game/Assets/3DMeshes/Enemy/EnemieAnimations/EnemyAttack/AM_EnemieAttack_full.AM_EnemieAttack_full" 1.0 "None")
            (Utilities|FlowControl|Delay 2.0)
            (bind _returnvalue (Game|SpawnActorfromClass "/Game/Assets/BluePrints/BP_EnemyProjectile.BP_EnemyProjectile_C" (Transformation|GetWorldTransform (Variables|Default|GetProjectileSpawner)) "Undefined" 0 0))
            (Physics|AddImpulse (Variables|/Game/Assets/BluePrints/BP_EnemyProjectile.BP_EnemyProjectile_C|GetSphere _returnvalue) (* (Math|Vector|GetForwardVector (Variables|Default|GetProjectileSpawner)) (* (Variables|Default|GetShootAmount) (/ (Transformation|GetDistanceTo (stale OnSeePawn(PawnSensing) Pawn)) 2.0))) "None" true)
            (Variables|Default|SetCanShootPlayer false)
            (Utilities|FlowControl|Delay 1.0)
            (Variables|Default|SetCanShootPlayer true)
            (Animation|StopAnimMontage "/Game/Assets/3DMeshes/Enemy/EnemieAnimations/EnemyAttack/AM_EnemieAttack_full.AM_EnemieAttack_full")
            (Utilities|FlowControl|Delay (Math|Random|RandomFloatinRange 0.5 1.0))
            (goto _label Reset)))))))

(event Custom|Follow%20Player
  (if (Variables|Default|GetIsSeeingPlayer)
    (AI|AIMoveTo self "0, 0, 0" (Game|GetPlayerCharacter 0) 5.0 false)))

(event Custom|Enemy%20Take%20Dmg
  (params (DMG%20taken :type Float%20%28double-precision%29))
  ;[0 1 0.04717] Enemy health
  (Variables|Default|SetEnemyHealth (- (Variables|Default|GetEnemyHealth) DMG%20taken))
  (if (<= (Variables|Default|GetEnemyHealth) 0.0)
    (CallFunction|EnemyDeath)
    (else
      (Animation|PlayAnimMontage "/Game/Assets/3DMeshes/Enemy/EnemieAnimations/Damadge/AM_One_damage.AM_One_damage" 1.0 "None"))))

(event Custom|Run%20From%20Player
  (AI|AIMoveTo self "0, 0, 0" (Game|GetPlayerCharacter 0) 5.0 false))

(event Custom|Enemy%20Gain%20HP
  (params (HP%20gained :type Float%20%28double-precision%29))
  ;[0 1 0.04717] Enemy health
  (Variables|Default|SetEnemyHealth (+ (Variables|Default|GetEnemyHealth) HP%20gained)))

(event Custom|Enemy%20Death
  ;[1 0 0.03249] EnemyDeath
  (Utilities|FlowControl|DoOnce false
    (:Completed
      (CallFunction|EnemyDropHead)
      (Pawn|Components|CharacterMovement|DisableMovement (Variables|Character|GetCharacterMovement))
      (Variables|Default|SetIsSeeingPlayer false)
      (Variables|Default|SetCanShootPlayer false)
      (Utilities|FlowControl|Delay 0.85)
      (Actor|DestroyActor))))

(event Custom|Enemy%20Drop%20Head
  (Rendering|SetVisibility (Variables|Character|GetMesh) false false)
  (Rendering|SetVisibility (Variables|Default|Getenemy_all_pieces_EnemyOneArm3R) true false)
  (Physics|SetSimulatePhysics (Variables|Default|Getenemy_all_pieces_EnemyOneBody) true)
  (Game|SpawnActorfromClass "/Game/Assets/BluePrints/BP_EnemyHead.BP_EnemyHead_C" (Transformation|GetWorldTransform (Variables|Default|GetHeadSpawner)) "Undefined" 0 0))

(event Custom|Face%20Player
  ;[1 1 1] Point twords player
  (Transformation|SetActorRotation (Math|Rotator|MakeRotator 0.0 0.0 (.yaw (Math|Interpolation|RInterpTo (Transformation|GetActorRotation) (Math|Rotator|FindLookatRotation (Transformation|GetActorLocation) (Transformation|GetActorLocation (stale OnSeePawn(PawnSensing) Pawn))) (Utilities|Time|GetWorldDeltaSeconds) 2e+01))))
  (Utilities|FlowControl|Delay 0.001)
  (CallFunction|FacePlayer))

(fn ConstructionScript)