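; BP_FireballSpawner is an actor that rains fireballs from above the player character.
; Every Tick it moves itself to a point high above player 0, so the spawn area follows the player.
; A looping timer started on BeginPlay periodically spawns a BP_FireBall2 at a random horizontal offset within a square around the spawner, at the spawner's height.
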(event Custom|Fireballs
  (bind _returnvalue (Transformation|GetActorLocation))
  (bind _output_get (Variables|Default|SetEnemySpawnLocation (Math|Vector|MakeVector (+ (.x _returnvalue) (Math|Random|RandomFloatinRange -6e+02 6e+02)) (+ (.y _returnvalue) (Math|Random|RandomFloatinRange -6e+02 6e+02)) (.z _returnvalue))))
  (Game|SpawnActorfromClass "/Game/Assets/BluePrints/BP_FireBall2.BP_FireBall2_C" (Math|Conversions|ToTransform(Vector) _output_get) "Undefined" 0 0))

(event EventBeginPlay
  (Utilities|Time|SetTimerbyEvent (delegate Custom|Fireballs) 2.0 true))

(event EventTick
  (params (DeltaSeconds :type Float%20%28single-precision%29))
  (bind _returnvalue (Game|GetPlayerCharacter 0))
  (bind _returnvalue_2 (Transformation|GetActorLocation _returnvalue))
  (Transformation|SetActorTransform (Math|Conversions|ToTransform(Vector) (Math|Vector|MakeVector (.x _returnvalue_2) (.y _returnvalue_2) (+ (.z _returnvalue_2) 1e+03)))))

(fn ConstructionScript)