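; Breakable wall Blueprint using a Chaos geometry collection that clears itself away after being broken by an enemy head.
; A box overlap with BP_EnemyHead arms the wall for removal.
; A later Chaos break event then removes the box and sets the player capsule to ignore the Destructible channel.
; After a short delay, it destroys the geometry collection and the actor.
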(event OnChaosBreakEvent(GeometryCollectionComponent)
  (params (BreakEvent :type Chaos%20Break%20Event%20Structure%20%28by%20ref%29))
  (if (Variables|Default|GetCan%20Disapear)
    (Components|DestroyComponent (Variables|Default|GetBox))
    (bind _asbp_third_person_character (Utilities|Casting|CastToBP_ThirdPersonCharacter (Game|GetPlayerCharacter 0)))
    (Collision|SetCollisionResponsetoChannel (Variables|/Script/Engine.Character|GetCapsuleComponent _asbp_third_person_character) "ECC_Destructible" "ECR_Ignore")
    (Utilities|FlowControl|Delay 3.0)
    (Components|DestroyComponent (Variables|Default|GetGeometryCollectionComponent))
    (Actor|DestroyActor)))

(event OnComponentBeginOverlap(Box)
  (params (OverlappedComponent :type Primitive%20Component%20Object%20Reference) (OtherActor :type Actor%20Object%20Reference) (OtherComp :type Primitive%20Component%20Object%20Reference) (OtherBodyIndex :type Integer) (bFromSweep :type Boolean) (SweepResult :type Hit%20Result%20Structure%20%28by%20ref%29))
  (Utilities|Casting|CastToBP_EnemyHead OtherActor)
  (Variables|Default|SetCan%20Disapear true))

(event EventBeginPlay)

(event Collision|EventActorBeginOverlap
  (params (OtherActor :type Actor%20Object%20Reference)))

(event EventTick
  (params (DeltaSeconds :type Float%20%28single-precision%29)))

(fn ConstructionScript)