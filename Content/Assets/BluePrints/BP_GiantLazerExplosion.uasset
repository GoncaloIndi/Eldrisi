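; BP_GiantLazerExplosion is a one-shot explosion that breaks and scatters Chaos destructible geometry, apparently walls.
; Its LazerWalls event spawns an explosion particle effect and sound, applies physics fields, then destroys the actor.
; A radial-falloff external strain field sized by the Sphere component fractures the geometry, then a culled radial-vector velocity field throws the pieces outward.
; BeginPlay is empty, so LazerWalls needs an external trigger.
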(event Custom|Lazer%20Walls
  (bind _returnvalue (Transformation|GetActorLocation))
  (bind _fieldsystemcomponent (Variables|Field|GetFieldSystemComponent))
  (bind _radialfalloff (Variables|Default|GetRadialFalloff))
  (bind _sphere (Variables|Default|GetSphere))
  (bind _returnvalue_2 (Transformation|GetWorldLocation _sphere))
  (bind _returnvalue_3 (Components|Sphere|GetScaledSphereRadius _sphere))
  (bind _returnvalue_4 (Field|SetRadialFalloff _radialfalloff 5e+05 0.0 1.0 0.0 _returnvalue_3 _returnvalue_2 "Field_FallOff_None"))
  (Effects|SpawnEmitteratLocation "/Game/StarterContent/Particles/P_Explosion.P_Explosion" _returnvalue "0, 0, 0" "3.000000,3.000000,3.000000")
  (Class|FMODBlueprintStatics|PlayEventatLocation "/Game/FMOD/Events/Giant/Explosion_3.Explosion_3" (Math|Conversions|ToTransform(Vector) _returnvalue))
  (Class|FieldSystemComponent|ApplyPhysicsField _fieldsystemcomponent true "Field_ExternalClusterStrain" 0 _returnvalue_4)
  (Class|FieldSystemComponent|ApplyPhysicsField _fieldsystemcomponent true "Field_LinearVelocity" 0 (Field|SetCullingField (Variables|Default|GetCullingField) _returnvalue_4 (Field|SetRadialVector (Variables|Default|GetRadialVector) 5e+02 _returnvalue_2) "Field_Culling_Outside"))
  (Actor|DestroyActor))

(event EventBeginPlay)

(fn ConstructionScript)