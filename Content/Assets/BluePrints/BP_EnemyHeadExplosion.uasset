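; Enemy head explosion actor that shatters and flings Chaos-destructible walls when ExplodeWalls is called.
; It activates a particle effect, plays an explosion sound event and triggers a world camera shake.
; Radial physics fields centered on its Sphere apply external cluster strain to break pieces, then culled linear velocity to push them outward.
; It destroys itself after a short delay; nothing in its own graph triggers the explosion.
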(event Custom|Explode%20Walls
  (bind _fieldsystemcomponent (Variables|Field|GetFieldSystemComponent))
  (bind _radialfalloff (Variables|Default|GetRadialFalloff))
  (bind _sphere (Variables|Default|GetSphere))
  (bind _returnvalue (Transformation|GetWorldLocation _sphere))
  (bind _returnvalue_2 (Components|Sphere|GetScaledSphereRadius _sphere))
  (bind _returnvalue_3 (Field|SetRadialFalloff _radialfalloff 5e+05 0.0 1.0 0.0 _returnvalue_2 _returnvalue "Field_FallOff_None"))
  (Components|Activation|Activate (Variables|Default|GetP_Explosion) false)
  (Class|FMODBlueprintStatics|PlayEventatLocation "/Game/FMOD/Events/Lvl_city/Explosion_2.Explosion_2" (Math|Conversions|ToTransform(Vector) (Transformation|GetActorLocation)))
  (Class|FieldSystemComponent|ApplyPhysicsField _fieldsystemcomponent true "Field_ExternalClusterStrain" 0 _returnvalue_3)
  (Class|FieldSystemComponent|ApplyPhysicsField _fieldsystemcomponent true "Field_LinearVelocity" 0 (Field|SetCullingField (Variables|Default|GetCullingField) _returnvalue_3 (Field|SetRadialVector (Variables|Default|GetRadialVector) 5e+02 _returnvalue) "Field_Culling_Outside"))
  (Camera|PlayWorldCameraShake "/Game/Assets/BluePrints/CameraShakesAndSoundMixer/BP_CameraShakeExplosion.BP_CameraShakeExplosion_C" (Transformation|GetActorLocation) 0.0 3e+03)
  (Utilities|FlowControl|Delay 2.0)
  (Actor|DestroyActor))

(event EventBeginPlay)

(fn ConstructionScript)