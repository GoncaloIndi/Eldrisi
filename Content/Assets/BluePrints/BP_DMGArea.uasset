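; BP_DMGArea is a damage area that hurts BP_ThirdPersonCharacter and knocks it back on contact.
; Two capsules each trigger their own DoOnce on begin overlap, dealing damage and launching the character upward and opposite its facing direction.
; Only the first capsule's end overlap resets both gates, and the trailing Delay in each branch leads to nothing.
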(event OnComponentBeginOverlap(Capsule1)
  (params (OverlappedComponent :type Primitive%20Component%20Object%20Reference) (OtherActor :type Actor%20Object%20Reference) (OtherComp :type Primitive%20Component%20Object%20Reference) (OtherBodyIndex :type Integer) (bFromSweep :type Boolean) (SweepResult :type Hit%20Result%20Structure%20%28by%20ref%29))
  (Utilities|FlowControl|DoOnce false
    (:Completed
      (bind _asbp_third_person_character (Utilities|Casting|CastToBP_ThirdPersonCharacter OtherActor))
      (Default|PlayerTakeDamadge _asbp_third_person_character 1.0)
      (Character|LaunchCharacter _asbp_third_person_character (Math|Vector|MakeVector (* (.x (Transformation|GetActorForwardVector _asbp_third_person_character)) -5.5e+02) (* (.y (Transformation|GetActorForwardVector _asbp_third_person_character)) -5.5e+02) 5e+02) true true)
      (Utilities|FlowControl|Delay 0.5))))

(event OnComponentBeginOverlap(Capsule)
  (params (OverlappedComponent :type Primitive%20Component%20Object%20Reference) (OtherActor :type Actor%20Object%20Reference) (OtherComp :type Primitive%20Component%20Object%20Reference) (OtherBodyIndex :type Integer) (bFromSweep :type Boolean) (SweepResult :type Hit%20Result%20Structure%20%28by%20ref%29))
  (Utilities|FlowControl|DoOnce false
    (:Completed
      (bind _asbp_third_person_character (Utilities|Casting|CastToBP_ThirdPersonCharacter OtherActor))
      (Default|PlayerTakeDamadge _asbp_third_person_character 1.0)
      (Character|LaunchCharacter _asbp_third_person_character (Math|Vector|MakeVector (* (.x (Transformation|GetActorForwardVector _asbp_third_person_character)) -5.5e+02) (* (.y (Transformation|GetActorForwardVector _asbp_third_person_character)) -5.5e+02) 5e+02) true true)
      (Utilities|FlowControl|Delay 0.5))))

(event OnComponentEndOverlap(Capsule)
  (params (OverlappedComponent :type Primitive%20Component%20Object%20Reference) (OtherActor :type Actor%20Object%20Reference) (OtherComp :type Primitive%20Component%20Object%20Reference) (OtherBodyIndex :type Integer))
  (Utilities|FlowControl|Sequence
    (:then_0
      (Utilities|FlowControl|DoOnce false) ; enters at Reset
    )
    (:then_1
      (Utilities|FlowControl|DoOnce false) ; enters at Reset
    )))

(fn ConstructionScript)