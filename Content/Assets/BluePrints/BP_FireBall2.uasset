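; Falling fireball hazard that damages the player on contact, with FMOD audio added on BeginPlay.
; Sphere1 overlap loops over the other actor's tags: Player takes damage, and any tag triggers impact unless a non-Landscape/Player/Enemy tag belongs to a spawner or fellow fireball.
; Impact destroys the collision, light and falling effects, activates Niagara, plays an FMOD impact sound, then destroys the actor after a short delay.
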(event OnComponentBeginOverlap(Sphere1)
  (params (OverlappedComponent :type Primitive%20Component%20Object%20Reference) (OtherActor :type Actor%20Object%20Reference) (OtherComp :type Primitive%20Component%20Object%20Reference) (OtherBodyIndex :type Integer) (bFromSweep :type Boolean) (SweepResult :type Hit%20Result%20Structure%20%28by%20ref%29))
  (for _array_element (Variables|/Script/Engine.Actor|GetTags OtherActor)
    (if (== _array_element "Landscape")
      _
      (elif (== _array_element "Player")
        (bind _asbp_third_person_character (Utilities|Casting|CastToBP_ThirdPersonCharacter OtherActor))
        (Default|PlayerTakeDamadge _asbp_third_person_character 1.0)
        (elif (== _array_element "Enemy")
          _
          (else
            (Utilities|Casting|CastToBP_FireballSpawner OtherActor
              (:CastFailed
                (Utilities|Casting|CastToBP_FireBall2 OtherActor
                  (:CastFailed
                    _))))))))
    (Components|DestroyComponent (Variables|Default|GetSphere1))
    (Components|Activation|Activate (Variables|Default|GetNiagara) false)
    (Class|FMODBlueprintStatics|PlayEventatLocation "/Game/Fmod/Events/Enemy_1/Fireball_Impact.Fireball_Impact" (Math|Conversions|ToTransform(Vector) (Transformation|GetWorldLocation (Variables|Default|GetSphere))))
    (Utilities|FlowControl|Delay 1.0)
    (Actor|DestroyActor)))

(event EventBeginPlay
  (AddComponent|AddFMODAudioComponent false))

(fn ConstructionScript)