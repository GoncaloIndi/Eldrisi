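; BP_GIANT is a giant enemy that turns to face the player and fires a laser after watching them long enough.
; PawnSensing rotates it while area events allow, and a one-second timer counts watch time, then starts the charge and later a cooldown.
; While firing, a gated Tick line-traces forward, steering a particle beam and spawning BP_GiantLazerExplosion once per hit.
; Older montage, damage and Niagara logic is left disconnected.
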(event OnSeePawn(PawnSensing)
  (params (Pawn :type Pawn%20Object%20Reference))
  ;[0 0.859 1] Visão
  (Utilities|Casting|CastToBP_ThirdPersonCharacter Pawn)
  (if (Variables|Giant|GetCan%20Look%20At%20Player)
    (Transformation|SetActorRotation (Math|Rotator|FindLookatRotation (Transformation|GetActorLocation) (Transformation|GetActorLocation (stale Custom|Player%20Is%20In%20Area player))))
    (Variables|Giant|SetLooking%20At%20Player true)))

(event Custom|ShootLazer
  (bind _returnvalue (Transformation|GetActorLocation))
  (bind _arrow1 (Variables|Default|GetArrow1))
  (bind _returnvalue_2 (Math|Vector|GetForwardVector _arrow1))
  (bind _returnvalue_3 (* _returnvalue_2 1.5e+03))
  (bind _returnvalue_4 (+ _returnvalue_3 _returnvalue))
  ;[1 0.05658 0] Lazer
  (Utilities|FlowControl|Gate true) ; enters at Open
)

(event Custom|Stop%20Lazer
  (bind _returnvalue (Transformation|GetActorLocation))
  (bind _arrow1 (Variables|Default|GetArrow1))
  (bind _returnvalue_2 (Math|Vector|GetForwardVector _arrow1))
  (bind _returnvalue_3 (* _returnvalue_2 1.5e+03))
  (bind _returnvalue_4 (+ _returnvalue_3 _returnvalue))
  ;[1 0.05658 0] Lazer
  (CallFunction|ResetLazer)
  (Variables|Giant|SetCan%20Look%20At%20Player true)
  (Utilities|FlowControl|Gate true) ; enters at Close
)

(event Custom|Charge%20Lazer
  ;[1 0.05658 0] Lazer
  (Variables|Giant|SetCan%20Look%20At%20Player false)
  (Utilities|FlowControl|Delay 3.0)
  (CallFunction|ShootLazer)
  (CallFunction|LazerDuration))

(event Custom|Player%20Is%20In%20Area
  (params (player :type Actor%20Object%20Reference))
  ;[0 0.859 1] Visão
  (Variables|Giant|SetCan%20Look%20At%20Player true))

(event Custom|Player%20Is%20Not%20In%20Area
  ;[0 0.859 1] Visão
  (Variables|Giant|SetCan%20Look%20At%20Player false)
  (Variables|Giant|SetPlayer%20Time%20In%20Vision 0.0)
  (Variables|Giant|SetLooking%20At%20Player false))

(event Custom|Player%20Is%20In%20vision%20Loop
  (bind _player_time_in_vision (Variables|Giant|GetPlayer%20Time%20In%20Vision))
  ;[1 0.2766 0] Comment
  (Utilities|Time|SetTimerbyEvent (delegate Custom|Player%20Is%20In%20vision%20Loop) 1.0 true)
  (if (Variables|Giant|GetLooking%20At%20Player)
    (if (Variables|Default|GetCan%20Attack)
      (Math|Float|IncrementFloat (Variables|Giant|GetPlayer%20Time%20In%20Vision)
        (:%20%20
          (if (>= _player_time_in_vision 6.0)
            (Variables|Default|SetPlayer%20Position%20For%20Lazer (Transformation|GetActorLocation (stale Custom|Player%20Is%20In%20Area player)))
            (CallFunction|ChargeLazer)
            (Variables|Default|SetCan%20Attack false)
            (else
              (Development|PrintString (Utilities|String|ToString(Float) _player_time_in_vision))))))
      (else
        ;;[1 1 1] Attack Cooldown
        (Utilities|FlowControl|Delay 15.0)
        (Variables|Default|SetCan%20Attack true)))))

(event Custom|Lazer%20Duration
  ;[1 0.05658 0] Lazer
  (Utilities|FlowControl|Delay 5.0)
  (CallFunction|StopLazer))

(event Custom|Reset%20Lazer
  ;[1 0.05658 0] Lazer
  (Utilities|FlowControl|Sequence
    (:then_0
      (Utilities|IsValid (Variables|Default|GetSystem)
        (:Is%20Valid
          (Components|Activation|Deactivate (Variables|Default|GetSystem))
          (Utilities|FlowControl|DoOnce false) ; enters at Reset
        )))
    (:then_1
      (Utilities|FlowControl|DoOnce false) ; enters at Reset
    )))

(event EventTick
  (params (DeltaSeconds :type Float%20%28single-precision%29))
  (bind _returnvalue (Transformation|GetActorLocation))
  (bind _arrow1 (Variables|Default|GetArrow1))
  (bind _returnvalue_2 (Math|Vector|GetForwardVector _arrow1))
  (bind _returnvalue_3 (* _returnvalue_2 1.5e+03))
  (bind _returnvalue_4 (+ _returnvalue_3 _returnvalue))
  ;[1 0.05658 0] Lazer
  (Utilities|FlowControl|Gate true
    (:Exit
      (Development|PrintString "Hello")
      (Variables|Default|SetPlayer%20Position%20For%20Lazer _returnvalue_4)
      (bind (_outhit _returnvalue_5) (Collision|LineTraceByChannel _returnvalue _returnvalue_4 "TraceTypeQuery1" false 0 "Persistent"))
      (if _returnvalue_5
        (Utilities|FlowControl|Sequence
          (:then_0
            (Utilities|FlowControl|DoOnce false
              (:Completed
                (bind _returnvalue_6 (Niagara|SpawnSystemAttached "/Game/Assets/Niagra/P_Lazer.P_Lazer" (Variables|Default|GetArrow1) "None" "0, 0, 0" "0, 0, 0" "SnapToTarget" false))
                (Variables|Default|SetSystem _returnvalue_6)
                (Utilities|FlowControl|DoOnce false
                  (:Completed
                    (bind _returnvalue_7 (Game|SpawnActorfromClass "/Game/Assets/BluePrints/BP_GiantLazerExplosion.BP_GiantLazerExplosion_C" (Math|Transform|MakeTransform (.location _outhit) "0, 0, 0" "1.000000,1.000000,1.000000") "Undefined" 0 0))
                    (Default|LazerWalls _returnvalue_7))))))
          (:then_1
            (Utilities|IsValid (Variables|Default|GetSystem)
              (:Is%20Valid
                (Effects|Components|ParticleSystem|SetVectorParameter (Variables|Default|GetSystem) "LOC" (.location _outhit))
                (if (> (Math|Vector|Distance(Vector) (.location _outhit) (Variables|Default|GetOut%20Hit%20Location)) 5e+01)
                  _)))))
        (else
          (CallFunction|ResetLazer))))))

(event EventBeginPlay
  ;[1 0.2766 0] Comment
  (CallFunction|PlayerIsinVisionLoop))

(fn ConstructionScript)