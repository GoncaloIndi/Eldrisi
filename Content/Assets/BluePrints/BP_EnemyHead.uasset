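; Enemy head that acts as a timed bomb: on spawn it lets the player pick up, then explodes after a short fuse.
; The blast sphere-traces the radial force radius, fires an impulse and damages the player, doubling the impulse if the player is holding.
; It then spawns BP_EnemyHeadExplosion to explode walls and destroys itself.
; Tick floats a camera-facing widget above the sphere, hidden while the player is holding.
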(event Custom|Explode
  (bind _sphere (Variables|Default|GetSphere))
  (bind _radialforce (Variables|Default|GetRadialForce))
  (bind _returnvalue (Transformation|GetWorldLocation _sphere))
  (bind _outhits (Collision|MultiSphereTraceForObjects _returnvalue _returnvalue (Variables|/Script/Engine.RadialForceComponent|GetRadius (Variables|Default|GetRadialForce)) (Variables|Default|GetObject%20Types%20Afected%20by%20explosion) false 0 "None"))
  (for _array_element _outhits
    (bind _asbp_third_person_character (Utilities|Casting|CastToBP_ThirdPersonCharacter (.hitactor _array_element)))
    (if (Variables|/Game/Assets/BluePrints/BP_ThirdPersonCharacter.BP_ThirdPersonCharacter_C|GetIsHolding? _asbp_third_person_character)
      (Variables|/Script/Engine.RadialForceComponent|SetImpulseStrength _radialforce 3e+03)
      (Class|RadialForceComponent|FireImpulse _radialforce)
      (Variables|/Script/Engine.RadialForceComponent|SetImpulseStrength _radialforce 1.5e+03)
      (Default|PlayerTakeDamadge _asbp_third_person_character 1.0)
      (else
        (Class|RadialForceComponent|FireImpulse _radialforce)
        (Default|PlayerTakeDamadge _asbp_third_person_character 1.0)))))

(event EventBeginPlay
  (bind _asbp_third_person_character (Utilities|Casting|CastToBP_ThirdPersonCharacter (Game|GetPlayerCharacter 0)))
  (Variables|/Game/Assets/BluePrints/BP_ThirdPersonCharacter.BP_ThirdPersonCharacter_C|SetCan%20Pick%20Up _asbp_third_person_character true)
  (Utilities|FlowControl|Delay 4.0)
  (CallFunction|Explode)
  (bind _returnvalue (Game|SpawnActorfromClass "/Game/Assets/BluePrints/BP_EnemyHeadExplosion.BP_EnemyHeadExplosion_C" (Math|Transform|MakeTransform (Transformation|GetWorldLocation (Variables|Default|GetSphere)) "0, 0, 0" "1.000000,1.000000,1.000000") "Undefined" 0 0))
  (Default|ExplodeWalls _returnvalue)
  (Actor|DestroyActor))

(event EventTick
  (params (DeltaSeconds :type Float%20%28single-precision%29))
  (bind _pivot_widget (Variables|Default|GetPivot%20widget))
  (bind _sphere (Variables|Default|GetSphere))
  (bind _returnvalue (Transformation|GetWorldLocation _sphere))
  (if (Variables|/Game/Assets/BluePrints/BP_ThirdPersonCharacter.BP_ThirdPersonCharacter_C|GetIsHolding? (stale EventBeginPlay _asbp_third_person_character))
    (Rendering|SetVisibility (Variables|Default|GetWidget) false false)
    (else
      (Transformation|SetWorldRotation _pivot_widget (Math|Rotator|FindLookatRotation (Transformation|GetActorLocation) (Transformation|GetWorldLocation (Variables|/Game/Assets/BluePrints/BP_ThirdPersonCharacter.BP_ThirdPersonCharacter_C|GetFollowCamera (stale EventBeginPlay _asbp_third_person_character)))) false false)
      (Transformation|SetWorldLocation _pivot_widget (Math|Vector|MakeVector (.x _returnvalue) (.y _returnvalue) (+ (.z _returnvalue) 7e+01)) false false)
      (Rendering|SetVisibility (Variables|Default|GetWidget) true false))))

(fn ConstructionScript)