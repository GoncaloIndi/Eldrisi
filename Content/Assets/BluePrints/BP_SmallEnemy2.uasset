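; BP_SmallEnemy2 is a melee enemy that chases and attacks the player, then spawns a detachable head actor on death.
; Pawn sensing starts a self-repeating delayed facing loop and an AI move that triggers attacks on arrival.
; A DoOnce-gated attack alternates two montages, then box-traces for damage unless a recent hit interrupts it.
; Tick pins a sphere to the neck socket and halts movement until the player is seen.
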(event OnSeePawn(PawnSensing)
  (params (Pawn :type Pawn%20Object%20Reference))
  (Variables|Default|SetIsSeeingPlayer true)
  (CallFunction|FacePlayer)
  (CallFunction|FollowPlayer))

(event Custom|Attack%20Player
  (bind _box (Variables|Default|GetBox))
  (bind _returnvalue (Transformation|GetWorldLocation _box))
  (if (not (Variables|Default|GetTaking%20Dmg))
    (Utilities|FlowControl|DoOnce false :!label _label
      (:Completed
        (if (Variables|Default|GetCanAttackPlayer)
          (Pawn|Components|CharacterMovement|DisableMovement (Variables|Character|GetCharacterMovement))
          ;[1 1 1] Shoot
          (Utilities|FlowControl|FlipFlop
            (:A
              (Animation|PlayAnimMontage "/Game/Assets/3DMeshes/Enemy/EnemieAnimations/Enemy2Attack1/One_attack__melee_Montage.One_attack__melee_Montage" 1.0 "None"))
            (:B
              (Animation|PlayAnimMontage "/Game/Assets/3DMeshes/Enemy/EnemieAnimations/Enemy2Attack2/one_melee2_Montage.one_melee2_Montage" 1.0 "None")))
          (AddComponent|AddFMODAudioComponent false)
          (Utilities|FlowControl|Delay 1.0)
          (if (Variables|Default|GetTaking%20Dmg)
            (Pawn|Components|CharacterMovement|SetMovementMode (Variables|Character|GetCharacterMovement) "MOVE_Walking" 0)
            (else
              (bind _outhit (Class|KismetSystemLibrary|BoxTraceSingleforObjects _returnvalue (- _returnvalue "0,0,0.100000") "100.000000,60.000000,100.000000" (Transformation|GetWorldRotation _box) (Utilities|Array|MakeArray "ObjectTypeQuery9") false 0 "None" true))
              (bind _asbp_third_person_character (Utilities|Casting|CastToBP_ThirdPersonCharacter (.HitActor (Collision|BreakHitResult _outhit)))
                (:then
                  (Default|PlayerTakeDamadge _asbp_third_person_character 3.0)
                  (Variables|Default|SetCanAttackPlayer false))
                (:CastFailed
                  _))
              (Utilities|FlowControl|Delay 1.75)
              (Variables|Default|SetCanAttackPlayer true)
              (Animation|StopAnimMontage "/Game/Assets/3DMeshes/Enemy/EnemieAnimations/Enemy2Attack1/One_attack__melee_Montage.One_attack__melee_Montage")
              (Utilities|FlowControl|Delay (Math|Random|RandomFloatinRange 0.5 1.0))
              (Pawn|Components|CharacterMovement|SetMovementMode (Variables|Character|GetCharacterMovement) "MOVE_Walking" 0)
              (goto _label Reset))))))))

(event Custom|Follow%20Player
  ;[1 1 1] Follow player
  (if (Variables|Default|GetIsSeeingPlayer)
    (AI|AIMoveTo self "0, 0, 0" (Game|GetPlayerCharacter 0) 1e+02 false
      (:OnSuccess
        (CallFunction|AttackPlayer)))
    (else
      (Variables|Default|SetIsSeeingPlayer false))))

(event Custom|Enemy%20Take%20Dmg
  (params (DMG%20taken :type Float%20%28double-precision%29))
  (bind _box (Variables|Default|GetBox))
  (bind _returnvalue (Transformation|GetWorldLocation _box))
  ;[0 1 0.04717] Enemy health
  (Variables|Default|SetEnemyHealth (- (Variables|Default|GetEnemyHealth) DMG%20taken))
  (if (<= (Variables|Default|GetEnemyHealth) 0.0)
    (CallFunction|EnemyDeath)
    (else
      (AddComponent|AddFMODAudioComponent false)
      (Animation|PlayAnimMontage "/Game/Assets/3DMeshes/Enemy/EnemieAnimations/Damadge/AM_One_damage.AM_One_damage" 1.0 "None")
      (Components|Activation|Activate (Variables|Default|GetP_Enemy2DeathSparks) true)
      (Variables|Default|SetTaking%20Dmg true)
      (Utilities|FlowControl|Delay 1.0)
      (Variables|Default|SetTaking%20Dmg false)
      (Utilities|FlowControl|DoOnce false) ; enters at Reset
    )))

(event Custom|Face%20Player
  ;[1 1 1] Face player
  (Transformation|SetActorRotation (Math|Rotator|MakeRotator 0.0 0.0 (.yaw (Math|Interpolation|RInterpTo (Transformation|GetActorRotation) (Math|Rotator|FindLookatRotation (Transformation|GetActorLocation) (Transformation|GetActorLocation (stale OnSeePawn(PawnSensing) Pawn))) (Utilities|Time|GetWorldDeltaSeconds) 2e+01))))
  (Utilities|FlowControl|Delay 0.001)
  (CallFunction|FacePlayer))

(event Custom|Enemy%20Gain%20HP
  (params (HP%20gained :type Float%20%28double-precision%29))
  ;[0 1 0.04717] Enemy health
  (Variables|Default|SetEnemyHealth (+ (Variables|Default|GetEnemyHealth) HP%20gained)))

(event Custom|Enemy%20Death
  ;[1 0 0.03249] EnemyDeath
  (Utilities|FlowControl|DoOnce false
    (:Completed
      (CallFunction|EnemyDropHead)
      (Pawn|Components|CharacterMovement|DisableMovement (Variables|Character|GetCharacterMovement))
      (Variables|Default|SetIsSeeingPlayer false)
      (Variables|Default|SetCanAttackPlayer false)
      (Actor|DestroyActor))))

(event Custom|Enemy%20Drop%20Head
  (Rendering|SetVisibility (Variables|Character|GetMesh) false false)
  (Game|SpawnActorfromClass "/Game/Assets/BluePrints/BP_EnemyHead.BP_EnemyHead_C" (Transformation|GetActorTransform self) "Undefined" 0 0))

(event EventTick
  (params (DeltaSeconds :type Float%20%28single-precision%29))
  (bind _sphere (Variables|Default|GetSphere))
  (bind _returnvalue (Transformation|GetWorldTransform _sphere))
  (Transformation|SetWorldTransform _sphere (Math|Transform|MakeTransform (.location (Transformation|GetSocketTransform (Variables|Character|GetMesh) "NeckJoint" "RTS_World")) (.rotation _returnvalue) (.scale _returnvalue)) false false)
  (if (not (Variables|Default|GetIsSeeingPlayer))
    (Components|Movement|StopMovementImmediately (Variables|Character|GetCharacterMovement))))

(fn ConstructionScript)